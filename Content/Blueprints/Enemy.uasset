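; Paper2D enemy character that takes damage and deals melee damage to overlapping players.
; AnyDamage lowers Health, playing a damage flipbook or, at zero, setting a death flipbook and immediately destroying the actor.
; Tick enters a DoOnce on sprite frame 3 while a player overlaps Box, triggering HitCheck to set the attack flipbook and apply BaseDamage.
; ResetAttack re-arms that DoOnce, and UpdateWalkSpeed sets movement speed.
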(event `self.ReceiveAnyDamage`
  (params (Damage :type "Float (single-precision)") (DamageType :type "DamageType Object Reference") (InstigatedBy :type "Controller Object Reference") (DamageCauser :type "Actor Object Reference"))
  (set `self.Health` (- (`self.Health`) Damage))
  (if (<= (`self.Health`) 0.0)
    (`PaperFlipbookComponent.SetFlipbook` (`self.Sprite`) "/Game/GameAssets/Flipbooks/Death_Enemy1.Death_Enemy1")
    (`PaperFlipbookComponent.SetLooping` (`self.Sprite`) false)
    (`self.K2_DestroyActor`)
    (else
      (`PaperFlipbookComponent.SetFlipbook` (`self.Sprite`) "/Game/GameAssets/Flipbooks/Damage_Eenemy1.Damage_Eenemy1")
      (`PaperFlipbookComponent.SetLooping` (`self.Sprite`) false))))

(event `ResetAttack`
  (goto _label :!via `Reset`))

(event `self.ReceiveTick`
  (params (DeltaSeconds :type "Float (single-precision)"))
  (for _ (`PrimitiveComponent.GetOverlappingActors` (`self.Box`) "/Game/Blueprints/PlayerBP.PlayerBP_C")
    (if (== (`PaperFlipbookComponent.GetPlaybackPositionInFrames` (`self.Sprite`)) 3)
      (`/Engine/EditorBlueprintResources/StandardMacros.DoOnce` false :!label _label
        (:`Completed`
          (`self.HitCheck`))))))

(fn `HitCheck`
  (for _array_element (`PrimitiveComponent.GetOverlappingActors` (`self.Box`) "/Game/Blueprints/PlayerBP.PlayerBP_C")
    (if (!= _array_element self)
      (`PaperFlipbookComponent.SetFlipbook` (`self.Sprite`) "/Game/GameAssets/Flipbooks/Attack_Enemy1.Attack_Enemy1")
      (`GameplayStatics.ApplyDamage` _array_element (`self.Base Damage`)))))

(fn `UpdateWalkSpeed`
  (params (NewWalkSpeed :type "Float (double-precision)"))
  (set `CharacterMovementComponent.MaxWalkSpeed` NewWalkSpeed (`self.CharacterMovement`)))

(fn `UserConstructionScript`)