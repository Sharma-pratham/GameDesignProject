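; Player character Blueprint for a side-scrolling 2D knight with Enhanced Input movement, jump and attack.
; Input and damage events swap the sprite's flipbooks, and movement direction flips the sprite.
; Attacking arms a DoOnce that Tick fires on flipbook frame 3, so HitCheck damages Enemy actors overlapping the Box.
; Each hit increments EnemyKillCount without a death check; zero Health shows the failure screen and destroys the actor.
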(event `self.ReceiveBeginPlay`
  (bind _asplayer_controller (cast `PlayerController` (`self.GetController`)))
  (`EnhancedInputSubsystemInterface.AddMappingContext` (pcsubsystem `EnhancedInputLocalPlayerSubsystem` _asplayer_controller) "/Game/Blueprints/IMC_SideScroller.IMC_SideScroller" 0 (struct)))

(event `EnhancedInput|/Game/Blueprints/Player_Movement`
  (params (ActionValue :type "Float (double-precision)") (ElapsedSeconds :type "Float (double-precision)") (TriggeredSeconds :type "Float (double-precision)") (InputAction :type "InputAction Object Reference" :default "/Game/Blueprints/Player_Movement.Player_Movement"))
  (:`Triggered`
    (`self.AddMovementInput` (1.0 0.0 0.0) ActionValue)
    (`PaperFlipbookComponent.SetFlipbook` (`self.Sprite`) "/Game/GameAssets/Flipbooks/Run_Knight.Run_Knight")
    (if (> ActionValue 0.0)
      (`SceneComponent.K2_SetWorldRotation` :`self` (`self.Sprite`))
      (else
        (`SceneComponent.K2_SetWorldRotation` (`self.Sprite`) (struct :`Yaw` -180.0) false false))))
  (:`Completed`
    (`PaperFlipbookComponent.SetFlipbook` (`self.Sprite`) "/Game/GameAssets/Flipbooks/Idle_knight.Idle_knight")))

(event `EnhancedInput|/Game/Blueprints/PlayerAttack`
  (params (ActionValue :type "Float (double-precision)") (ElapsedSeconds :type "Float (double-precision)") (TriggeredSeconds :type "Float (double-precision)") (InputAction :type "InputAction Object Reference" :default "/Game/Blueprints/PlayerAttack.PlayerAttack"))
  (:`Started`
    (`PaperFlipbookComponent.SetFlipbook` (`self.Sprite`) "/Game/GameAssets/Flipbooks/Attack_Knight.Attack_Knight"))
  (:`Completed`
    (`PaperFlipbookComponent.SetFlipbook` (`self.Sprite`) "/Game/GameAssets/Flipbooks/Idle_knight.Idle_knight")))

(event `EnhancedInput|/Game/Blueprints/Player_Jump`
  (params (ActionValue :type "Float (double-precision)") (ElapsedSeconds :type "Float (double-precision)") (TriggeredSeconds :type "Float (double-precision)") (InputAction :type "InputAction Object Reference" :default "/Game/Blueprints/Player_Jump.Player_Jump"))
  (bind _sprite (`self.Sprite`))
  (:`Triggered`
    (`self.Jump`)
    (`PaperFlipbookComponent.SetLooping` _sprite false)
    (`PaperFlipbookComponent.SetFlipbook` _sprite "/Game/GameAssets/Flipbooks/Jump_Knight.Jump_Knight")
    (if (== (`.Z` (`KismetMathLibrary.BreakVector3f` (`self.GetVelocity`))) 0.0)
      (`PaperFlipbookComponent.SetLooping` _sprite true)
      (`PaperFlipbookComponent.Play` _sprite)
      (`PaperFlipbookComponent.SetFlipbook` (`self.Sprite`) "/Game/GameAssets/Flipbooks/Idle_knight.Idle_knight")))
  (:`Canceled`
    (`PaperFlipbookComponent.SetFlipbook` (`self.Sprite`) "/Game/GameAssets/Flipbooks/Idle_knight.Idle_knight")))

(event `EnhancedInput|/Game/Blueprints/PlayerAttack`
  (params (ActionValue :type "Float (double-precision)") (ElapsedSeconds :type "Float (double-precision)") (TriggeredSeconds :type "Float (double-precision)") (InputAction :type "InputAction Object Reference" :default "/Game/Blueprints/PlayerAttack.PlayerAttack"))
  (:`Started`
    (`PaperFlipbookComponent.SetFlipbook` (`self.Sprite`) "/Game/GameAssets/Flipbooks/Attack_Knight.Attack_Knight")
    (`PaperFlipbookComponent.SetLooping` (`self.Sprite`) false)
    (set `self.isAttacking` true)
    (`self.ResetAttack`)
    (`SceneComponent.SetHiddenInGame` (`self.Box`) false false)))

(event `self.Sprite.OnFinishedPlaying`
  (`PaperFlipbookComponent.SetFlipbook` (`self.Sprite`) "/Game/GameAssets/Flipbooks/Idle_knight.Idle_knight")
  (`PaperFlipbookComponent.SetLooping` (`self.Sprite`) false)
  (if (not (`PaperFlipbookComponent.IsPlaying` (`self.Sprite`)))
    (`PaperFlipbookComponent.Play` (`self.Sprite`))))

(event `ResetAttack`
  (goto _label :!via `Reset`))

(event `self.ReceiveTick`
  (params (DeltaSeconds :type "Float (single-precision)"))
  (if (`self.isAttacking`)
    (if (== (`PaperFlipbookComponent.GetPlaybackPositionInFrames` (`self.Sprite`)) 3)
      (`/Engine/EditorBlueprintResources/StandardMacros.DoOnce` false :!label _label
        (:`Completed`
          (`self.HitCheck`))))
    (else
      (`SceneComponent.SetHiddenInGame` (`self.Box`) true false))))

(event `self.ReceiveAnyDamage`
  (params (Damage :type "Float (single-precision)") (DamageType :type "DamageType Object Reference") (InstigatedBy :type "Controller Object Reference") (DamageCauser :type "Actor Object Reference"))
  (set `self.Health` (- (`self.Health`) Damage))
  (if (<= (`self.Health`) 0.0)
    (bind _returnvalue (`|CreateWidget` "/Game/Widgets/FailureScreen.FailureScreen_C"))
    (`UserWidget.AddToViewport` _returnvalue 0)
    (`PaperFlipbookComponent.SetFlipbook` (`self.Sprite`) "/Game/GameAssets/Flipbooks/Death_Knight.Death_Knight")
    (`PaperFlipbookComponent.SetLooping` (`self.Sprite`) false)
    (`self.K2_DestroyActor`)
    (else
      (`PaperFlipbookComponent.SetFlipbook` (`self.Sprite`) "/Game/GameAssets/Flipbooks/Damage_Knight.Damage_Knight")
      (`PaperFlipbookComponent.SetLooping` (`self.Sprite`) false))))

(fn `HitCheck`
  (for _array_element (`PrimitiveComponent.GetOverlappingActors` (`self.Box`) "/Game/Blueprints/Enemy.Enemy_C")
    (if (!= _array_element self)
      (`GameplayStatics.ApplyDamage` _array_element (`self.Base Damage`))
      (if true
        (bind _output_get (set `self.EnemyKillCount` (+ (`self.EnemyKillCount`) 1.0)))))))

(fn `UserConstructionScript`)